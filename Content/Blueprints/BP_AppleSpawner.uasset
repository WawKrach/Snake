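; BP_AppleSpawner keeps apples coming by spawning a BP_Apple at a random free spot in the play area.
; Candidate points come from a box sized by VerticalSpace and HorizontalSpace and are rejected if an apple-sized sphere trace hits something.
; After a short random delay it spawns at a clear point, retrying periodically when blocked.
; Each apple's AppleEated dispatcher triggers the next spawn.
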(event Custom|SpawnApple
  (Utilities|FlowControl|Delay (Math|Random|RandomFloatinRange 1.0 2.0))
  (bind (_returnvalue _spacefound) (CallFunction|TrytoFindSpaceforNewApple :!label _label))
  (if _spacefound
    (bind _returnvalue_2 (Game|SpawnActorfromClass "/Game/Blueprints/BP_Apple.BP_Apple_C" (Math|Transform|MakeTransform _returnvalue "0, 0, 0" (.StartScale (Utilities|GetClassDefaults "/Game/Blueprints/BP_Apple.BP_Apple_C"))) "Undefined" 0 0))
    (EventDispatchers|AssignAppleEated _returnvalue_2 (delegate Custom|AppleEated_Dispatcher))
    (else
      (Utilities|FlowControl|Delay 0.5)
      (goto _label))))

(event Custom|AppleEated_Dispatcher
  (CallFunction|SpawnApple))

(event EventBeginPlay
  (CallFunction|SpawnApple))

(fn ConstructionScript)

(fn TrytoFindSpaceforNewApple
  (bind _output_get (LocalVariables|SetPossibleSpawnLocation (Math|Random|RandomPointinBoundingBox "0.000000,0.000000,50.000000" (Math|Vector|MakeVector (Variables|Default|GetVerticalSpace) (Variables|Default|GetHorizontalSpace) 0.1))))
  (bind _returnvalue (Collision|SphereTraceByChannel _output_get (+ _output_get 0.1) (.AppleSphereSize (Utilities|GetClassDefaults "/Game/Blueprints/BP_Apple.BP_Apple_C")) "TraceTypeQuery1" false 0 "None"))
  (if (not _returnvalue)
    (return (LocalVariables|GetPossibleSpawnLocation) true)
    (else
      (return "0, 0, 0" false))))