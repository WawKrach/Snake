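; Player pawn for a Snake game that spawns and steers the snake head and creates the score widget.
; Tick turns movement axes into a direction, passing changes to the head unless they nearly reverse the last one.
; Head events for eaten apples and death are relayed through score and reset dispatchers.
; Death also destroys all body segments and apples, then respawns the head after a delay.
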(event Custom|ResetSnake
  ;[0 1 0.08209] Reset snake
  (Utilities|FlowControl|Sequence
    (:then_0
      (bind _outactors (Actor|GetAllActorsOfClass "/Game/Blueprints/BP_SnakeBody.BP_SnakeBody_C"))
      (for _array_element _outactors
        (Actor|DestroyActor _array_element))
      (bind _outactors_2 (Actor|GetAllActorsOfClass "/Game/Blueprints/BP_Apple.BP_Apple_C"))
      (for _array_element_2 _outactors_2
        (Actor|DestroyActor _array_element_2)))
    (:then_1
      (Utilities|FlowControl|Delay 2.0)
      (CallFunction|SpawnSnakeHead))))

(event Custom|SpawnSnakeHead
  ;[0 1 0.285] Spawn snake head
  (bind _returnvalue (Game|SpawnActorfromClass "/Game/Blueprints/BP_SnakeHead.BP_SnakeHead_C" (Math|Transform|MakeTransform "0, 0,50.000000" "0, 0, 0" "1,1,1") "AlwaysSpawn" 0 8e+01 "0.000000,0.000000,0.000000" 8e+01 0 0 0))
  (bind _output_get (Variables|Default|SetSneakHead _returnvalue))
  (EventDispatchers|BindEventtoAppleEated _output_get (delegate Custom|ScoreApple))
  (EventDispatchers|BindEventtoSnakeDie _output_get (delegate Custom|ResetGame)))

(event Custom|ScoreApple
  (params (Score :type Integer))
  ;[0 1 0.285] Spawn snake head
  (Default|CallUpdateScore Score))

(event Custom|ResetGame
  ;[0 1 0.285] Spawn snake head
  (CallFunction|ResetSnake)
  (Default|CallGameReset))

(event EventTick
  (params (DeltaSeconds :type Float%20%28single-precision%29))
  (bind _sneakhead (Variables|Default|GetSneakHead))
  ;[0 1 0.3939] Controll snake head
  (Utilities|IsValid _sneakhead
    (:Is%20Valid
      ;;[0.1827 1 0.01481] Get input
      (bind (_rotation _direction _change) (CallFunction|ChangeSnakeDirection))
      (if (not _change)
        (if (Math|Vector|NotEqual(Vector) (Variables|Default|GetLastDirection) _direction 0.0001)
          ;;[0.1827 1 0.01481] Set direction
          (Default|SetNewDirection _sneakhead _direction _rotation)
          (Variables|Default|SetLastDirection _direction))))))

(event EventBeginPlay
  (CallFunction|SpawnSnakeHead)
  (bind _returnvalue (UserInterface|CreateWidget "/Game/Blueprints/W_Scores.W_Scores_C" (Game|GetPlayerController 0)))
  (bind _output_get (Variables|Default|SetScoreWidget _returnvalue))
  (UserInterface|Viewport|AddtoViewport _output_get 0))

(fn ConstructionScript
  (Transformation|DetachFromComponent (Variables|Default|GetCamera) "KeepWorld" "KeepWorld" "KeepRelative" true))

(fn ChangeSnakeDirection
  (bind _returnvalue (Utilities|Time|GetWorldDeltaSeconds))
  (bind _returnvalue_2 (Input|AxisValues|GetMoveVertical))
  (bind _returnvalue_3 (Input|AxisValues|GetMoveHorizontal))
  (bind _inputforce (Variables|Default|GetInputForce))
  (bind _returnvalue_4 (Math|Vector|MakeVector _returnvalue_2 _returnvalue_3 0.0))
  (bind _returnvalue_5 (* _returnvalue _inputforce))
  (bind _returnvalue_6 (Math|Vector|ClampVectorSize _returnvalue_4 0.0 1.0))
  (bind _returnvalue_7 (* _returnvalue_6 _returnvalue_5))
  (if (> (Math|Vector|VectorLength _returnvalue_7) 0.0)
    (return (Math|Conversions|RotationFromXVector _returnvalue_7) _returnvalue_7 (Math|Vector|Equal(Vector) (Variables|Default|GetLastDirection) (* _returnvalue_7 -1.0) 1.0))))