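; Snake body segment actor that trails the part ahead and can spawn the next one at its tail, registering it with the Head.
; It follows queued turn points, passing each to the next segment once crossed, and adds distance-based catch-up speed to close gaps.
; When flagged, it wraps across level bounds by mirroring X or Y, holding incoming turns until teleported, then flags the next segment.
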(event Custom|SetNewDirection
  (params (NewDirection :type Vector) (Rotation :type Rotator))
  ;[0 1 0.2812] Movement
  (Variables|Movement|SetDirection NewDirection)
  (Transformation|SetWorldRotation (Variables|Default|GetDefaultSceneRoot) Rotation false false))

(event Custom|SetNextRoutePoint
  (params (RoutePoint :type Struct%20Route%20Point%20Structure))
  ;[0 1 0.2812] Movement
  (if (Variables|Teleport|GetGoingToTeleport)
    (Utilities|Array|Add (Variables|Teleport|GetWaitingForTeleportRoutePoints) RoutePoint)
    (else
      (Utilities|Array|Add (Variables|Movement|GetRoutePoints) RoutePoint))))

(event Custom|SpawnNextBodyPart
  (bind _head (Variables|Default|GetHead))
  ;[0 1 0.6202] Spawn next body part
  (Utilities|FlowControl|DoOnce false
    (:Completed
      (Utilities|IsValid _head
        (:Is%20Valid
          (bind _returnvalue (Game|SpawnActorfromClass "BP_SnakeBody_C" (Transformation|GetWorldTransform (Variables|Default|GetTailEnd)) "AlwaysSpawn" 0 (Variables|Movement|GetDirection) (Variables|Movement|GetMovementSpeed) _head self 0))
          (bind _output_get (Variables|Default|SetNextBodyPart _returnvalue))
          (Utilities|Array|Add (Variables|/Game/Blueprints/BP_SnakeHead.BP_SnakeHead_C|GetBodyParts _head) _output_get))))))

(event Custom|Teleport
  (params (NewLocation :type Vector))
  (bind _nextbodypart (Variables|Default|GetNextBodyPart))
  (bind _waitingforteleportroutepoints (Variables|Teleport|GetWaitingForTeleportRoutePoints))
  ;[0 1 0.3537] Teleport
  (Variables|Teleport|SetGoingToTeleport false)
  (Transformation|SetActorLocation NewLocation true true)
  (if (> (Utilities|Array|Length (Variables|Teleport|GetWaitingForTeleportRoutePoints)) 0)
    (Utilities|Array|AppendArray (Variables|Movement|GetRoutePoints) _waitingforteleportroutepoints)
    (Utilities|Array|Clear _waitingforteleportroutepoints))
  (Utilities|IsValid _nextbodypart
    (:Is%20Valid
      (Variables|BP_SnakeBody_C|SetGoingToTeleport _nextbodypart true))))

(event EventBeginPlay)

(event EventTick
  (params (DeltaSeconds :type Float%20%28single-precision%29))
  ;[0 1 0.2812] Movement
  (Utilities|FlowControl|Sequence
    (:then_0
      (if (.Valid (Movement|GetCurrentRoutePoint))
        (if (Movement|CheckRoutePointPass)
          (Movement|RouteDirection)
          (else
            (Movement|MoveSnakeBodyPart :!label _label)))
        (else
          (goto _label))))
    (:then_1
      (if (Variables|Teleport|GetGoingToTeleport)
        (bind (_teleport _teleportlocation) (Teleport|CheckTeleporting))
        (if _teleport
          (CallFunction|Teleport _teleportlocation))))))

(fn ConstructionScript)

(fn MoveSnakeBodyPart
  (Utilities|IsValid (Variables|Default|GetPrevBodyPart)
    (:Is%20Valid
      (Transformation|AddActorWorldOffset (* (Variables|Movement|GetDirection) (+ (* (Variables|Movement|GetMovementSpeed) (Utilities|Time|GetWorldDeltaSeconds)) (Math|Float|MapRangeClamped (Math|Vector|VectorLength (- (Transformation|GetActorLocation (Variables|Default|GetPrevBodyPart)) (Transformation|GetActorLocation))) 5e+01 7e+01 0.0 (/ (* (/ (Variables|Movement|GetMovementSpeed) 8e+01) (/ (Variables|Movement|GetMovementSpeed) 8e+01)) 2.0)))) true))
    (:Is%20Not%20Valid
      (Transformation|AddActorWorldOffset (* (Variables|Movement|GetDirection) (* (Variables|Movement|GetMovementSpeed) (Utilities|Time|GetWorldDeltaSeconds))) true))))

(fn CheckRoutePointPass
  (bind _routepoint (Movement|GetCurrentRoutePoint))
  (return (or (or (and (> (.y (Variables|Movement|GetDirection)) 0.0) (< (.y _routepoint) (.y (Transformation|GetActorLocation)))) (and (< (.y (Variables|Movement|GetDirection)) 0.0) (> (.y _routepoint) (.y (Transformation|GetActorLocation))))) (or (and (> (.x (Variables|Movement|GetDirection)) 0.0) (< (.x _routepoint) (.x (Transformation|GetActorLocation)))) (and (< (.x (Variables|Movement|GetDirection)) 0.0) (> (.x _routepoint) (.x (Transformation|GetActorLocation))))))))

(fn GetCurrentRoutePoint
  (bind _routepoints (Variables|Movement|GetRoutePoints))
  (bind _returnvalue (Utilities|Array|Length _routepoints))
  (bind _returnvalue_2 (> _returnvalue 0))
  (if _returnvalue_2
    (return (.RoutePoint (Utilities|Struct|BreakStruct_RoutePoint (Utilities|Array|Get(acopy) _routepoints))) _returnvalue_2)
    (else
      (return "0, 0, 0" false))))

(fn RouteDirection
  (bind _routepoints (Variables|Movement|GetRoutePoints))
  (bind _nextbodypart (Variables|Default|GetNextBodyPart))
  (bind _output (Utilities|Array|Get(acopy) _routepoints))
  (bind _newdirection (Utilities|Struct|BreakStruct_RoutePoint _output))
  (CallFunction|SetNewDirection _newdirection (Math|Conversions|RotationFromXVector _newdirection))
  (Utilities|FlowControl|Sequence
    (:then_0
      (Utilities|IsValid _nextbodypart
        (:Is%20Valid
          (CallFunction|SetNextRoutePoint _nextbodypart (Utilities|Array|Get(acopy) (Variables|Movement|GetRoutePoints))))))
    (:then_1
      (Utilities|Array|RemoveIndex (Variables|Movement|GetRoutePoints)))))

(fn CheckTeleporting
  (bind _returnvalue (Transformation|GetActorLocation))
  (bind _returnvalue_2 (Transformation|GetActorLocation))
  (if (> (Math|Float|Absolute(Float) (.x (Transformation|GetActorLocation))) (Variables|Teleport|GetMaxVerticalLocationX))
    (bind _output_get (LocalVariables|SetTargetLocation (Math|Vector|MakeVector (* (.x _returnvalue) -1.0) (.y _returnvalue) (.z _returnvalue))))
    (return true _output_get)
    (elif (> (Math|Float|Absolute(Float) (.y (Transformation|GetActorLocation))) (Variables|Teleport|GetMaxHorizontalLocationY))
      (bind _output_get_2 (LocalVariables|SetTargetLocation (Math|Vector|MakeVector (.x _returnvalue_2) (* (.y _returnvalue_2) -1.0) (.z _returnvalue_2))))
      (return true _output_get_2)
      (else
        (return false "0.000000,0.0,0.0")))))

(fn IncreaseSpeed
  (Variables|Movement|SetMovementSpeed (+ (Variables|Movement|GetMovementSpeed) (Variables|Movement|GetSpeedIncrease))))