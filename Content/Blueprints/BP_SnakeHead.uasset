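; Head segment of a snake game that moves each tick, teleports when needed, eats apples and detects self-collision.
; Direction changes pass a route point to the next body part so followers turn at the same spot.
; Overlapping an apple grows the tail, increases speed and score, and calls AppleEated.
; Overlapping a body segment other than the two nearest calls SnakeDie.
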(event OnComponentBeginOverlap(Sphere1)
  (params (OverlappedComponent :type Primitive%20Component%20Object%20Reference) (OtherActor :type Actor%20Object%20Reference) (OtherComp :type Primitive%20Component%20Object%20Reference) (OtherBodyIndex :type Integer) (bFromSweep :type Boolean) (SweepResult :type Hit%20Result%20Structure%20%28by%20ref%29))
  (bind _nextbodypart (Variables|Default|GetNextBodyPart))
  ;[0 1 0.255] Eat&Die
  (bind _asbp_apple (Utilities|Casting|CastToBP_Apple OtherActor)
    (:then
      (CallFunction|EatApple _asbp_apple))
    (:CastFailed
      (bind _asbp_snake_body (Utilities|Casting|CastToBP_SnakeBody OtherActor))
      (if (Math|Boolean|ANDBoolean (!= _asbp_snake_body _nextbodypart) (!= _asbp_snake_body self) (!= _asbp_snake_body (Variables|/Game/Blueprints/BP_SnakeBody.BP_SnakeBody_C|GetNextBodyPart _nextbodypart)))
        (Default|CallSnakeDie)))))

(event Custom|EatApple
  (params (Apple :type Actor%20Object%20Reference))
  (bind _output (CallFunction|GetLastBodyPart))
  ;[0 1 0.255] Eat&Die
  (Actor|DestroyActor Apple)
  (Utilities|IsValid _output
    (:Is%20Valid
      (Default|SpawnNextBodyPart _output)
      (CallFunction|IncreaseSpeed)
      (bind _result (Math|Integer|IncrementInt (Variables|Default|GetScores))
        (:%20%20
          (Default|CallAppleEated _result))))))

(event EventBeginPlay
  ;[0 1 0.5031] SnakeHead
  (bind _output_get (Variables|Default|SetHead self))
  (Utilities|Array|Add (Variables|Default|GetBodyParts) _output_get))

(event EventSetNewDirection
  (params (NewDirection :type Vector :default "0, 0, 0") (Rotation :type Rotator :default "0, 0, 0"))
  (bind _nextbodypart (Variables|Default|GetNextBodyPart))
  ;[0 1 0.5031] SnakeHead
  (|CallParentFunction NewDirection Rotation)
  ;;[0.9111 1 0] Set route point for next body part to change  direction
  (Utilities|IsValid _nextbodypart
    (:Is%20Valid
      (Default|SetNextRoutePoint _nextbodypart (Utilities|Struct|MakeStruct_RoutePoint (Transformation|GetActorLocation) (Variables|Default|GetDirection))))))

(event EventTick
  (params (DeltaSeconds :type Float%20%28single-precision%29))
  ;[0 1 0.5031] SnakeHead
  (CallFunction|MoveSnakeBodyPart)
  (bind (_teleport _teleportlocation) (CallFunction|CheckTeleporting))
  (if _teleport
    (CallFunction|Teleport _teleportlocation)))

(fn ConstructionScript
  (|CallParentFunction))

(fn GetLastBodyPart
  (bind _bodyparts (Variables|Default|GetBodyParts))
  (return (Utilities|Array|Get(acopy) _bodyparts (- (Utilities|Array|Length _bodyparts) 1))))